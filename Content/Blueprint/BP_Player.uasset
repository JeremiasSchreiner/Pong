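; BP_Player is the player's paddle in a Pong game, a Cube moved by Enhanced Input.
; BeginPlay casts the player controller to PC_PongController and adds the IMC_PongActions mapping context.
; IA_Movement offsets the Cube along local Y by the input value times Speed, then clamps its world X to fixed bounds.
; The offset is applied per triggered event, without delta-time scaling.
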(event `self.ReceiveBeginPlay`
  ;[1 1 1] Input mapping actions
  (bind _aspc_pong_controller (cast `/Game/Blueprint/PC_PongController` (`GameplayStatics.GetPlayerController` 0)))
  (bind _returnvalue (pcsubsystem `EnhancedInputLocalPlayerSubsystem` _aspc_pong_controller))
  (`/Engine/EditorBlueprintResources/StandardMacros.IsValid` _returnvalue
    (:`Is Valid`
      (`EnhancedInputSubsystemInterface.AddMappingContext` _returnvalue "/Game/Input/IMC_PongActions.IMC_PongActions" 0 (struct)))))

(event `EnhancedInput|/Game/Input/Input_Action/IA_Movement`
  (params (ActionValue :type "Float (double-precision)") (ElapsedSeconds :type "Float (double-precision)") (TriggeredSeconds :type "Float (double-precision)") (InputAction :type "InputAction Object Reference" :default "/Game/Input/Input_Action/IA_Movement.IA_Movement"))
  (bind _cube (`self.Cube`))
  (bind (_returnvalue_x _returnvalue_y _returnvalue_z) (`KismetMathLibrary.BreakVector` (`SceneComponent.K2_GetComponentLocation` _cube)))
  (:`Triggered`
    (`SceneComponent.K2_AddLocalOffset` (`self.Cube`) (`KismetMathLibrary.MakeVector` 0.0 (* ActionValue (`self.speed`))) false false)
    (`SceneComponent.K2_SetWorldLocation` _cube (`KismetMathLibrary.MakeVector` (`KismetMathLibrary.FClamp` _returnvalue_x -658.0 120.0) _returnvalue_y _returnvalue_z) false false)))

(fn `UserConstructionScript`)